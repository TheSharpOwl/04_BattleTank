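; Player-controllable tank pawn Blueprint with gimbal aiming, track movement, firing and a health bar.
; BeginPlay hands the barrel, turret and projectile class to TankAiming, the tracks to TankMovement, and the tank itself to the HealthBar widget.
; Input axes rotate the azimuth gimbal and spring arm scaled by delta time, or pass move intents to TankMovement.
; Fire calls TankAiming, and Swap Cam toggles first and third person cameras.
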(event Collision|EventActorBeginOverlap
  (params (OtherActor :type Actor%20Object%20Reference)))

(event EventBeginPlay
  (Variables|/Script/BattleTank.TankAimingComponent|SetProjectileBlueprint (Variables|Default|GetTankAiming) "/Game/Projectile/Projectile_BP.Projectile_BP_C")
  (Class|TankAimingComponent|Initialise (Variables|Default|GetTankAiming) (Variables|Default|GetTankBarrel) (Variables|Default|GetTankTurret))
  (Class|TankMovementComponent|Initialise (Variables|Default|GetTankMovement) (Variables|Default|GetLeftTrack) (Variables|Default|GetRightTrack))
  (CallFunction|InitializeHealthBarWidget))

(event Input|ActionEvents|InputActionSwapCam
  (params (Key :type Key%20Structure))
  ;[1 1 1] Camera Swap
  (:Pressed
    (Components|Activation|ToggleActive (Variables|Default|Get1st%20Person))
    (Components|Activation|ToggleActive (Variables|Default|Get3rd%20Person))))

(event Input|ActionEvents|InputActionFire
  (params (Key :type Key%20Structure))
  ;[1 1 1] Movement Input Binding
  (:Pressed
    (Class|TankAimingComponent|Fire (Variables|Default|GetTankAiming))))

(event Input|AxisEvents|InputAxisAimAzimuth
  (params (AxisValue :type Float%20%28single-precision%29))
  ;[1 1 1] Balistics Input Binding
  (Transformation|AddLocalRotation (Variables|Default|GetAzimuth%20Gimbal) (Math|Rotator|MakeRotator 0.0 0.0 (* AxisValue (Utilities|Time|GetWorldDeltaSeconds) 1e+02)) false false))

(event Input|AxisEvents|InputAxisMoveForward
  (params (AxisValue :type Float%20%28single-precision%29))
  ;[1 1 1] Movement Input Binding
  (Class|TankMovementComponent|IntendMoveForward (Variables|Default|GetTankMovement) AxisValue))

(event Input|AxisEvents|InputAxisAimElevation
  (params (AxisValue :type Float%20%28single-precision%29))
  ;[1 1 1] Balistics Input Binding
  (Transformation|AddLocalRotation (Variables|Default|GetSpringArm) (Math|Rotator|MakeRotator 0.0 (* AxisValue (Utilities|Time|GetWorldDeltaSeconds) 1e+02) 0.0) false false))

(event Input|AxisEvents|InputAxisTurnRight
  (params (AxisValue :type Float%20%28single-precision%29))
  ;[1 1 1] Movement Input Binding
  (Class|TankMovementComponent|IntendTurnRight (Variables|Default|GetTankMovement) AxisValue))

(fn ConstructionScript)

(fn InitializeHealthBarWidget
  (bind _ashealth_bar (Utilities|Casting|CastToHealthBar (UserInterface|GetUserWidgetObject (Variables|Default|GetWidget))))
  (Variables|/Game/UI/HealthBar.HealthBar_C|SetMyTank _ashealth_bar self))